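; BP_Player is a player Blueprint with unconnected logic for sprinting and landing camera feedback.
; The sprint chains swap walk speed between sprint and default, starting a stored camera shake when moving and stopping it on return to default.
; A landing chain plays a world camera shake at the player's location.
; None of these chains are wired to events, so OnLanded and the construction script do nothing.
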(event `self.OnLanded`
  (params (Hit :type "HitResult Structure (by ref)")))

(event `InputAction|Sprint`
  (params (Key :type "Key Structure")))

(fn `UserConstructionScript`)